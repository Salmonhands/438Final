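; Player controller for a lap-based vehicle race that owns the HUD, runs the click-started countdown and handles vehicle respawn and level restart.
; Timelines drive race and lap clocks, feeding HUD text and hiding gold, silver and bronze goals once missed.
; Lap updates check lap and final race records, play HUD animations and save bests to a SaveGame slot.
; The R key resets saved records to defaults outside a race.
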(event Custom|StartGameSetup
  ;[1 1 1] Start Game Sequence
  (CallFunction|SaveGameCheck)
  (CallFunction|InitText))

(event Custom|RespawnVehicle
  ;[1 1 1] Respawn when flipped
  (bind _returnvalue (Game|SpawnActorfromClass "/Game/VehicleAdvBP/Blueprints/VehicleBlueprint.VehicleBlueprint_C" (Variables|Default|GetRespawnLocation) "Undefined" 0 0))
  (Pawn|Possess _returnvalue))

(event Custom|StartRaceTime
  ;[1 1 1] Start/Stop Race/Lap Timers
  (bind _time (Timeline|GameTime Play)
    (:Update
      (bind _output_get (Variables|ValueVariables|SetActualRaceTime _time))
      (Variables|TextVariables|SetRaceTimeText (Utilities|TimetoText _output_get))
      (CallFunction|UpdateGoals))))

(event Custom|Restart
  ;[1 1 1] Restart Map when race is over
  (Variables|Default|SetRaceStart false)
  (Utilities|FlowControl|Delay 6.0)
  (Development|ExecuteConsoleCommand "RestartLevel"))

(event Custom|StopLapTime
  ;[1 1 1] Start/Stop Race/Lap Timers
  (bind _time (Timeline|LapTime Stop)
    (:Update
      (Variables|ValueVariables|SetActualLapTime _time))))

(event Custom|StopRaceTime
  ;[1 1 1] Start/Stop Race/Lap Timers
  (bind _time (Timeline|GameTime Stop)
    (:Update
      (bind _output_get (Variables|ValueVariables|SetActualRaceTime _time))
      (Variables|TextVariables|SetRaceTimeText (Utilities|TimetoText _output_get))
      (CallFunction|UpdateGoals))))

(event Custom|StartLapTime
  ;[1 1 1] Start/Stop Race/Lap Timers
  (bind _time (Timeline|LapTime PlayFromStart)
    (:Update
      (Variables|ValueVariables|SetActualLapTime _time))))

(event Custom|UpdateLap
  ;[1 1 1] Adds to current lap and checks for record
  (if (Variables|Default|GetRaceComplete)
    _
    (else
      (bind _output_get (Variables|ValueVariables|SetActualLap (+ (Variables|ValueVariables|GetActualLap) 1)))
      (bind _output_get_2 (Variables|TextVariables|SetCurrentLapText (Utilities|Text|ToText(Integer) _output_get)))))
  (CallFunction|LapTimeCheck)
  (Development|PrintText _output_get_2))

(event EventBeginPlay
  ;[1 1 1] Begin / Get References
  (bind _returnvalue (UserInterface|CreateWidget "/Game/Blueprints/UI/HUD.HUD_C"))
  (bind _output_get (Variables|Default|SetHUDReference _returnvalue))
  (UserInterface|Viewport|AddtoViewport _output_get 0)
  (bind _asvehicle_blueprint (Utilities|Casting|CastToVehicleBlueprint (Game|Player|GetPlayerPawn 0)))
  (Variables|Default|SetVehicleReference _asvehicle_blueprint))

(event Input|KeyboardEvents|R
  (params (Key :type Key%20Structure :default "AnyKey"))
  ;[1 1 1] R: reset to default times if not in race
  (:Pressed
    (if (not (Variables|Default|GetRaceStart))
      (Variables|ValueVariables|SetBestLapTime (Variables|ValueVariables|GetDefaultBestLapTime))
      (Variables|ValueVariables|SetBestRaceTime (Variables|ValueVariables|GetDefaultBestRaceTime))
      (CallFunction|SavetheGame)
      (CallFunction|InitText))))

(event Input|MouseEvents|LeftMouseButton
  (params (Key :type Key%20Structure :default "AnyKey"))
  (bind _hudreference (Variables|Default|GetHUDReference))
  (bind _hudreference_2 (Variables|Default|GetHUDReference))
  ;[1 1 1] Left Click: Start Race
  (:Pressed
    (Utilities|FlowControl|DoOnce false
      (:Completed
        (Variables|/Game/Blueprints/UI/HUD.HUD_C|SetSplashScreenVisible _hudreference "Hidden")
        (Variables|/Game/Blueprints/UI/HUD.HUD_C|SetCountDownVisible _hudreference "Visible")
        (UserInterface|Animation|PlayAnimation _hudreference (Variables|/Game/Blueprints/UI/HUD.HUD_C|GetCountDownAnimation _hudreference) 0.0 1 "Forward")
        (Utilities|FlowControl|Delay 2.5)
        (Variables|TextVariables|SetReadyText "2")
        (Utilities|FlowControl|Delay 1.0)
        (Variables|TextVariables|SetReadyText "1")
        (Utilities|FlowControl|Delay 1.0)
        (Variables|TextVariables|SetReadyText "Go!")
        (Utilities|FlowControl|Delay 1.0)
        (Variables|/Game/Blueprints/UI/HUD.HUD_C|SetCountDownVisible _hudreference_2 "Hidden")
        (Variables|/Game/Blueprints/UI/HUD.HUD_C|SetGameHUDVisible _hudreference_2 "Visible")
        (Variables|Default|SetRaceStart true)
        (CallFunction|StartRaceTime)
        (CallFunction|StartLapTime)))))

(fn ConstructionScript)

(fn InitText
  ;[1 1 1] Convert to numerical methods for HUD
  (Variables|TextVariables|SetCurrentLapText (Utilities|Text|ToText(Integer) (Variables|ValueVariables|GetActualLap)))
  (Variables|TextVariables|SetMaxLapText (Utilities|Text|ToText(Integer) (Variables|ValueVariables|GetMaxLaps)))
  (Variables|TextVariables|SetRaceTimeText (Utilities|TimetoText (Variables|ValueVariables|GetActualRaceTime)))
  (Variables|TextVariables|SetLapTimeText (Utilities|TimetoText (Variables|ValueVariables|GetActualLapTime)))
  (Variables|TextVariables|SetGoldTimeText (Utilities|TimetoText (Variables|ValueVariables|GetGoldTime)))
  (Variables|TextVariables|SetSilverTimeText (Utilities|TimetoText (Variables|ValueVariables|GetSilverTime)))
  (Variables|TextVariables|SetBronzeTimeText (Utilities|TimetoText (Variables|ValueVariables|GetBronzeTime)))
  (Variables|TextVariables|SetBestLapText (Utilities|TimetoText (Variables|ValueVariables|GetBestLapTime)))
  (Variables|TextVariables|SetBestTimeText (Utilities|TimetoText (Variables|ValueVariables|GetBestRaceTime))))

(fn SaveGameCheck
  ;[1 1 1] Loads a saved game if it exists or default game
  (bind _returnvalue (SaveGame|DoesSaveGameExist (Variables|Default|GetSaveSlot)))
  (if _returnvalue
    (CallFunction|LoadtheGame)
    (else
      (Variables|ValueVariables|SetBestLapTime (Variables|ValueVariables|GetDefaultBestLapTime))
      (Variables|ValueVariables|SetBestRaceTime (Variables|ValueVariables|GetDefaultBestRaceTime))
      (CallFunction|SavetheGame))))

(fn SavetheGame
  ;[1 1 1] Saves game to save slot
  (bind _returnvalue (SaveGame|CreateSaveGameObject "/Game/Blueprints/MySaveGame.MySaveGame_C"))
  (bind _output_get (LocalVariables|SetSavedGameReference _returnvalue))
  (bind _asmy_save_game (Utilities|Casting|CastToMySaveGame _output_get))
  (Variables|/Game/Blueprints/MySaveGame.MySaveGame_C|SetSavedBestLap _asmy_save_game (Variables|ValueVariables|GetBestLapTime))
  (Variables|/Game/Blueprints/MySaveGame.MySaveGame_C|SetSavedBestTime _asmy_save_game (Variables|ValueVariables|GetBestRaceTime))
  (SaveGame|SaveGametoSlot (LocalVariables|GetSavedGameReference) (Variables|Default|GetSaveSlot)))

(fn LoadtheGame
  ;[1 1 1] Loads the game
  (bind _returnvalue (SaveGame|LoadGamefromSlot (Variables|Default|GetSaveSlot)))
  (bind _asmy_save_game (Utilities|Casting|CastToMySaveGame _returnvalue))
  (Variables|ValueVariables|SetBestLapTime (Variables|/Game/Blueprints/MySaveGame.MySaveGame_C|GetSavedBestLap _asmy_save_game))
  (Variables|ValueVariables|SetBestRaceTime (Variables|/Game/Blueprints/MySaveGame.MySaveGame_C|GetSavedBestTime _asmy_save_game)))

(fn LapTimeCheck
  (bind _hudreference (Variables|Default|GetHUDReference))
  ;[1 1 1] Saves a new lap record if one was set, resets lap time
  (CallFunction|StopLapTime)
  (if (<= (Variables|ValueVariables|GetActualLapTime) (Variables|ValueVariables|GetBestLapTime))
    (bind _output_get (Variables|ValueVariables|SetBestLapTime (Variables|ValueVariables|GetActualLapTime)))
    (Variables|TextVariables|SetBestLapText (Utilities|TimetoText _output_get))
    (CallFunction|SavetheGame)
    (UserInterface|Animation|PlayAnimation _hudreference (Variables|/Game/Blueprints/UI/HUD.HUD_C|GetLapAnimation _hudreference) 0.0 1 "Forward"))
  (Variables|ValueVariables|SetActualLapTime 0.0)
  (if (Variables|Default|GetRaceComplete)
    (CallFunction|RaceTimeCheck)
    (else
      (CallFunction|StartLapTime))))

(fn RaceTimeCheck
  (bind _hudreference (Variables|Default|GetHUDReference))
  (CallFunction|StopRaceTime)
  (if (<= (Variables|ValueVariables|GetActualRaceTime) (Variables|ValueVariables|GetBestRaceTime))
    (bind _output_get (Variables|ValueVariables|SetBestRaceTime (Variables|ValueVariables|GetActualRaceTime)))
    (Variables|TextVariables|SetBestTimeText (Utilities|TimetoText _output_get))
    (UserInterface|Animation|PlayAnimation _hudreference (Variables|/Game/Blueprints/UI/HUD.HUD_C|GetRaceAnimation _hudreference) 0.0 1 "Forward")
    (CallFunction|SavetheGame)))

(fn UpdateGoals
  ;[1 1 1] Sets Goal Times to Hidden if no longer attainable
  (if (not (<= (Variables|ValueVariables|GetActualRaceTime) (Variables|ValueVariables|GetGoldTime)))
    (Utilities|FlowControl|Sequence
      (:then_0
        (Utilities|FlowControl|DoOnce false
          (:Completed
            (Variables|/Game/Blueprints/UI/HUD.HUD_C|SetGoldTimeVisible (Variables|Default|GetHUDReference) "Hidden"))))
      (:then_1
        (if (not (<= (Variables|ValueVariables|GetActualRaceTime) (Variables|ValueVariables|GetSilverTime)))
          (Utilities|FlowControl|Sequence
            (:then_0
              (Utilities|FlowControl|DoOnce false
                (:Completed
                  (Variables|/Game/Blueprints/UI/HUD.HUD_C|SetSilverTimeVisible (Variables|Default|GetHUDReference) "Hidden"))))
            (:then_1
              (if (not (<= (Variables|ValueVariables|GetActualRaceTime) (Variables|ValueVariables|GetBronzeTime)))
                (Utilities|FlowControl|DoOnce false
                  (:Completed
                    (Variables|/Game/Blueprints/UI/HUD.HUD_C|SetBronzeTimeVisible (Variables|Default|GetHUDReference) "Hidden")))))))))))